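; BP_Clouds is a cloud actor built around the NSClouds Niagara component, configurable through exposed parameters.
; Its Construction Script pushes particle size, spawn rate, opacity, white-particle reach and box size into the Niagara system.
; It also writes the white cloud origin to the shared MPC_Clouds material parameter collection.
; The Event Graph holds only disabled placeholder events, so the Blueprint has no runtime logic.
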(fn `UserConstructionScript`
  (`NiagaraComponent.SetVariableFloat` (`self.NS_Clouds`) "ParticlesSize" (`self.ParticlesSize`))
  (`NiagaraComponent.SetVariableFloat` (`self.NS_Clouds`) "SpawnRate" (`self.SpawnRate`))
  (`NiagaraComponent.SetVariableFloat` (`self.NS_Clouds`) "Opacity" (`self.Opacity`))
  (`NiagaraComponent.SetVariableFloat` (`self.NS_Clouds`) "WhiteParticleReach" (`self.WhiteParticles_Bounds`))
  (`NiagaraComponent.SetVariableVec3` (`self.NS_Clouds`) "BoxSize" (`self.BoxSize`))
  (`KismetMaterialLibrary.SetVectorParameterValue` "/Game/VFX/MPC_Clouds.MPC_Clouds" "WhiteParticlesOrigin" (`KismetMathLibrary.Conv_VectorToLinearColor` (`self.WhiteCloud_Origin`))))