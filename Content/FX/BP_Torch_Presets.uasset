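; Configurable torch and fire prop whose construction script builds one of several presets, from wall torches to candles, with no runtime logic.
; The preset sets mesh, flame particles (overridable) and component offsets.
; A light preset optionally enables a generic or light-function point light with exposed color, intensity, radius, offset and shadows.
; With a light enabled, the fake glow takes its color and gets randomized material parameters and scale for variation, or is destroyed if switched off.
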(event `self.ReceiveBeginPlay`)

(fn `UserConstructionScript`
  (bind _returnvalue (`KismetMathLibrary.RandomFloatInRange` 0.75 1.25))
  (bind _ps_largeflame (`self.PS_LargeFlame`))
  (bind _ps_smallflame (`self.PS_SmallFlame`))
  (bind _light_color (`self.Light_Color`))
  (bind _cast_shadows (`self.Cast_Shadows`))
  (`StaticMeshComponent.SetStaticMesh` (`self.SM_Torch`) (select `/Game/FX/Enum_TorchList` (`self.Presets`) :`NewEnumerator0` (`self.SM_StandingWood`) :`NewEnumerator1` (`self.SM_StoneHolder`) :`NewEnumerator2` (`self.SM_WallTorch`) :`NewEnumerator3` (`self.SM_TallMetal`) :`NewEnumerator4` (`self.SM_HangingMetal`) :`NewEnumerator5` (`self.SM_PileOfBones`) :`NewEnumerator6` (`self.SM_Candles`) :`NewEnumerator7` (`self.SM_Metal_Post`)))
  (`SceneComponent.SetRelativeScale3D` (`self.SM_Torch`) (select `/Game/FX/Enum_TorchList` (`self.Presets`) :`NewEnumerator0` (1.0 1.0 1.0) :`NewEnumerator1` (1.0 1.0 1.0) :`NewEnumerator2` (1.0 1.0 1.0) :`NewEnumerator3` (1.0 1.0 1.0) :`NewEnumerator4` (1.0 1.0 1.0) :`NewEnumerator5` (1.0 1.0 1.0) :`NewEnumerator6` (1.0 1.0 1.0) :`NewEnumerator7` (0.5 0.5 0.5) :!type "Vector Structure"))
  (if (`self.CustomParticle_Set`)
    (`ParticleSystemComponent.SetTemplate` (`self.PS_Fire`) (`self.PS_Particle_System`))
    (else
      (`ParticleSystemComponent.SetTemplate` (`self.PS_Fire`) (select `/Game/FX/Enum_TorchList` (`self.Presets`) :`NewEnumerator0` (`self.PS_MediumFlame`) :`NewEnumerator1` _ps_largeflame :`NewEnumerator2` _ps_smallflame :`NewEnumerator3` _ps_largeflame :`NewEnumerator4` _ps_largeflame :`NewEnumerator5` _ps_smallflame :`NewEnumerator6` (`self.PS_Candles`)))))
  (`SceneComponent.K2_SetRelativeLocation` (`self.PS_Fire`) (select `/Game/FX/Enum_TorchList` (`self.Presets`) :`NewEnumerator0` (0.0 0.0 90.0) :`NewEnumerator1` (0.0 0.0 58.0) :`NewEnumerator2` (0.0 15.0 45.0) :`NewEnumerator3` (0.0 0.0 156.0) :`NewEnumerator4` (0.0 0.0 -73.0) :`NewEnumerator7` (95.0 0.0 500.0) :!type "Vector Structure") false false)
  (`SceneComponent.K2_SetRelativeLocation` (`self.FakeGlow`) (select `/Game/FX/Enum_TorchList` (`self.Presets`) :`NewEnumerator0` (0.0 0.0 90.0) :`NewEnumerator1` (0.0 0.0 58.0) :`NewEnumerator2` (0.0 15.0 45.0) :`NewEnumerator3` (0.0 0.0 156.0) :`NewEnumerator4` (0.0 0.0 -73.0) :`NewEnumerator7` (95.0 0.0 500.0) :!type "Vector Structure") false false)
  (`SceneComponent.K2_SetRelativeLocation` (`self.SM_Torch`) (select `/Game/FX/Enum_TorchList` (`self.Presets`) :`NewEnumerator4` (0.0 0.0 75.0) :!type "Vector Structure") false false)
  (if (select `/Game/FX/Enum_TorchList_Lights` (`self.Light_Presets`) :`NewEnumerator1` true :`NewEnumerator2` true)
    (`SceneComponent.SetVisibility` (select `/Game/FX/Enum_TorchList_Lights` (`self.Light_Presets`) :`NewEnumerator1` (`self.PointLight_Generic`) :`NewEnumerator2` (`self.PointLight_WithMaterial`)) true false)
    (`SceneComponent.SetVisibility` (`self.FakeGlow`) true false)
    (`SceneComponent.K2_SetRelativeLocation` (select `/Game/FX/Enum_TorchList_Lights` (`self.Light_Presets`) :`NewEnumerator1` (`self.PointLight_Generic`) :`NewEnumerator2` (`self.PointLight_WithMaterial`)) (+ (select `/Game/FX/Enum_TorchList` (`self.Presets`) :`NewEnumerator0` (0.0 0.0 125.0) :`NewEnumerator1` (0.0 0.0 100.0) :`NewEnumerator2` (0.0 15.0 45.0) :`NewEnumerator3` (0.0 0.0 156.0) :`NewEnumerator4` (0.0 0.0 -73.0) :`NewEnumerator7` (95.0 0.0 500.0) :!type "Vector Structure") (`self.Light_Offset`)) false false)
    (`LightComponent.SetIntensity` (select `/Game/FX/Enum_TorchList_Lights` (`self.Light_Presets`) :`NewEnumerator1` (`self.PointLight_Generic`) :`NewEnumerator2` (`self.PointLight_WithMaterial`)) (`self.Light_Intensity`))
    (`LocalLightComponent.SetAttenuationRadius` (select `/Game/FX/Enum_TorchList_Lights` (`self.Light_Presets`) :`NewEnumerator1` (`self.PointLight_Generic`) :`NewEnumerator2` (`self.PointLight_WithMaterial`)) (`self.Light_Radius`))
    (`LightComponent.SetLightColor` (select `/Game/FX/Enum_TorchList_Lights` (`self.Light_Presets`) :`NewEnumerator1` (`self.PointLight_Generic`) :`NewEnumerator2` (`self.PointLight_WithMaterial`)) _light_color true)
    (if (`self.Fake_Glow`)
      (`MeshComponent.SetVectorParameterValueOnMaterials` (`self.FakeGlow`) "Color" (`KismetMathLibrary.Conv_LinearColorToVector` _light_color))
      (`MeshComponent.SetScalarParameterValueOnMaterials` (`self.FakeGlow`) "Randomize_Offset" (`KismetMathLibrary.RandomFloat`))
      (`MeshComponent.SetScalarParameterValueOnMaterials` (`self.FakeGlow`) "Randomize_Speed" (`KismetMathLibrary.RandomFloatInRange` -2.0 2.0))
      (`MeshComponent.SetScalarParameterValueOnMaterials` (`self.FakeGlow`) "Randomize_Tiling_U" (`KismetMathLibrary.Conv_IntToDouble` (`KismetMathLibrary.RandomIntegerInRange` 1 2)))
      (`MeshComponent.SetScalarParameterValueOnMaterials` (`self.FakeGlow`) "Randomize_Tiling_V" (`KismetMathLibrary.Conv_IntToDouble` (`KismetMathLibrary.RandomIntegerInRange` 1 2)))
      (`SceneComponent.SetRelativeScale3D` (`self.FakeGlow`) (* (`KismetMathLibrary.MakeVector` (* (`KismetMathLibrary.RandomFloatInRange` 0.75 1.25) _returnvalue) _returnvalue _returnvalue) (`self.Glow_Scale`)))
      (else
        (`ActorComponent.K2_DestroyComponent` (`self.FakeGlow`))))
    (if (select `/Game/FX/Enum_TorchList_Lights` (`self.Light_Presets`) :`NewEnumerator2` true)
      (`LightComponent.SetLightFunctionMaterial` (`self.PointLight_WithMaterial`) (`self.Light_Material`)))
    ;[1 1 1] Volmetric Scattering (Not currently using volumetric fog)
    (`LightComponent.SetVolumetricScatteringIntensity` (select `/Game/FX/Enum_TorchList_Lights` (`self.Light_Presets`) :`NewEnumerator1` (`self.PointLight_Generic`) :`NewEnumerator2` (`self.PointLight_WithMaterial`)) (`self.Volumetric_Scattering`))
    (`LightComponentBase.SetCastShadows` (`self.PointLight_Generic`) (select `/Game/FX/Enum_TorchList_Lights` (`self.Light_Presets`) :`NewEnumerator1` _cast_shadows :`NewEnumerator2` _cast_shadows))
    (`LightComponentBase.SetCastShadows` (`self.PointLight_WithMaterial`) (select `/Game/FX/Enum_TorchList_Lights` (`self.Light_Presets`) :`NewEnumerator1` _cast_shadows :`NewEnumerator2` _cast_shadows))))